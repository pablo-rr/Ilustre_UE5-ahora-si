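; Player controller that creates the player UI for the local player and passes their chosen class into the game session.
; On BeginPlay it reads the class from the game instance and relays it through server and multicast-named events into the player state.
; A separate PlayerConnect event, triggered by PlayerConnectedSERVER, copies each player state's class onto every custom hero actor.
; Debug prints show the class at both hand-off points.
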(event `self.ReceiveBeginPlay`
  (if (`self.IsLocalPlayerController`)
    (bind _returnvalue (`|CreateWidget` "/Game/UI/WG_PlayerUI.WG_PlayerUI_C"))
    (`UserWidget.AddToViewport` _returnvalue 0)
    (bind _asbp_my_game_instance (cast `/Game/Blueprints/GameplayFramework/BP_MyGameInstance` (`GameplayStatics.GetGameInstance`)))
    (bind _playerclass (`/Game/Blueprints/GameplayFramework/BP_MyGameInstance.playerClass` _asbp_my_game_instance))
    (`self.SetClassServer` _playerclass)
    (`KismetSystemLibrary.PrintString` (`|GetEnumeratorNameAsString` _playerclass))))

(event `SetClassServer`
  (params (ClaseServer :type "/Game/Blueprints/ENUM_Clases Enum" :default "NewEnumerator0"))
  (`self.SetClassMulticast` ClaseServer))

(event `SetClassMulticast`
  (params (ClaseMulticast :type "/Game/Blueprints/ENUM_Clases Enum" :default "NewEnumerator0"))
  (bind _asbp_my_player_state (cast `/Game/Blueprints/GameplayFramework/BP_MyPlayerState` (`self.PlayerState`)))
  (bind _output_get (set `/Game/Blueprints/GameplayFramework/BP_MyPlayerState.playerClass` ClaseMulticast _asbp_my_player_state))
  (`KismetSystemLibrary.PrintString` (`|GetEnumeratorNameAsString` _output_get)))

(event `PlayerConnect`
  (bind _outactors (`GameplayStatics.GetAllActorsOfClass` "/Game/Blueprints/Hero/BP_CustomHero.BP_CustomHero_C"))
  (for _array_element _outactors
    (bind _asbp_my_player_state (cast `/Game/Blueprints/GameplayFramework/BP_MyPlayerState` (`Pawn.PlayerState` _array_element)))
    (set `/Game/Blueprints/Hero/BP_CustomHero.Class` (`/Game/Blueprints/GameplayFramework/BP_MyPlayerState.playerClass` _asbp_my_player_state) _array_element)))

(event `PlayerConnectedSERVER`
  (`self.PlayerConnect`))

(fn `UserConstructionScript`)