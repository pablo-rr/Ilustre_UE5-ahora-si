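; Game State Blueprint that syncs each player's chosen class onto their in-game actor when a player connects.
; PlayerConnected calls SyncClassServer, which forwards to SyncclassMulri, names suggesting a server-to-multicast chain.
; That event finds all actors of the passed-in class, prints their count, and copies PlayerClass from each one's BP_MyPlayerState into the actor's Class variable.
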(event `SyncClassServer`
  (params (NewParam :type "/Game/Blueprints/Hero/BP_CustomHero Class Reference"))
  (`self.SyncclassMulri` NewParam))

(event `self.ReceiveBeginPlay`)

(event `PlayerConnected`
  (params (NewParam :type "/Game/Blueprints/Hero/BP_CustomHero Class Reference"))
  (`self.SyncClassServer` NewParam))

(event `SyncclassMulri`
  (params (NewParam :type "/Game/Blueprints/Hero/BP_CustomHero Class Reference"))
  (bind _outactors (`GameplayStatics.GetAllActorsOfClass` NewParam))
  (`KismetSystemLibrary.PrintString` (`KismetStringLibrary.Conv_IntToString` (`KismetArrayLibrary.Array_Length` _outactors)))
  (for _array_element _outactors
    (bind _asbp_my_player_state (cast `/Game/Blueprints/GameplayFramework/BP_MyPlayerState` (`Pawn.PlayerState` _array_element)))
    (set `/Game/Blueprints/Hero/BP_CustomHero.Class` (`/Game/Blueprints/GameplayFramework/BP_MyPlayerState.playerClass` _asbp_my_player_state) _array_element)))

(fn `UserConstructionScript`)