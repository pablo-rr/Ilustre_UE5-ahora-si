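; Player hero character for a networked sprite-based game, playable as Guardian, Warrior, Wizard or Archer, with OnRep_Class swapping the animation class.
; Attack and run inputs relay through server-to-multicast events: melee classes briefly enable attack collision, ranged classes spawn fireballs or arrows.
; Ability 1, handled locally, toggles a Wizard ability actor or fires a lit Archer arrow.
; It also handles planar movement, left/right facing, interaction and damage, with death only printed.
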(event `SetClassServer`
  (params (NewParam :type "/Game/Blueprints/ENUM_Clases Enum" :default "NewEnumerator0"))
  (`self.SetClassAll` NewParam))

(event `InputAction|Interact`
  (params (Key :type "Key Structure"))
  (:`Pressed`
    (for _array_element (`self.GetOverlappingActors` "/Script/Engine.Actor")
      (if (`KismetSystemLibrary.DoesImplementInterface` _array_element "/Game/Blueprints/1ev/BPI_PlayerActionable.BPI_PlayerActionable_C")
        (message `/Game/Blueprints/1ev/BPI_PlayerActionable.OnPlayerActivated` _array_element null)
        (break)))))

(event `SetClassAll`
  (params (NewParam :type "/Game/Blueprints/ENUM_Clases Enum" :default "NewEnumerator0"))
  (set `self.Class` NewParam))

(event `self.ReceiveBeginPlay`
  (`|ExecutionSequence`
    (:`then_0`
      (`self.EnableInput` (`GameplayStatics.GetPlayerController` 0)))
    (:`then_1`
      (set `self.RunSpeed` (* (`self.WalkSpeed`) 1.5)))
    (:`then_2`
      (`PrimitiveComponent.SetCollisionEnabled` (`self.AttackColision`) "NoCollision"))
    (:`then_3`
      (`KismetSystemLibrary.PrintString` (`KismetSystemLibrary.GetDisplayName` self)))))

(event `InputAction|Attack`
  (params (Key :type "Key Structure"))
  ;[1 1 1] Ataque Básico
  (:`Pressed`
    (`self.AttackServer`)))

(event `AttackServer`
  ;[1 1 1] Ataque Básico
  (`self.AttackMulticast`))

(event `AttackMulticast`
  (bind _attackcolision (`self.AttackColision`))
  (bind _shoot (`self.Shoot`))
  (bind _shoot_2 (`self.Shoot`))
  ;[1 1 1] Ataque Básico
  (switch `/Game/Blueprints/ENUM_Clases` (`self.Class`)
    (:`NewEnumerator0`
      (if (!= (`self.isAttacking`) true) :!label _label
        (set `self.isAttacking` true)
        (`PrimitiveComponent.SetCollisionEnabled` _attackcolision "QueryAndPhysics")
        (`KismetSystemLibrary.Delay` (`self.delayAttack`))
        (set `self.isAttacking` false)
        (`PrimitiveComponent.SetCollisionEnabled` _attackcolision "NoCollision")))
    (:`NewEnumerator1`
      (if (!= (`self.isAttacking`) true)
        (set `self.isAttacking` true)
        (`KismetSystemLibrary.Delay` 0.5)
        (`|SpawnActorFromClass` "/Game/Blueprints/Actors/BP_Fireball.BP_Fireball_C" (`KismetMathLibrary.MakeTransform` (`SceneComponent.K2_GetComponentLocation` _shoot) (`SceneComponent.K2_GetComponentRotation` _shoot)) "Undefined" "OverrideRootScale" null null)
        (`KismetSystemLibrary.Delay` 0.5)
        (set `self.isAttacking` false)))
    (:`NewEnumerator2`
      (if (!= (`self.isAttacking`) true)
        (set `self.isAttacking` true)
        (`KismetSystemLibrary.Delay` 0.5)
        (`|SpawnActorFromClass` "/Game/Blueprints/Actors/BP_Arrow.BP_Arrow_C" (`KismetMathLibrary.MakeTransform` (`SceneComponent.K2_GetComponentLocation` _shoot_2) (`SceneComponent.K2_GetComponentRotation` _shoot_2)) "Undefined" "OverrideRootScale" null null)
        (`KismetSystemLibrary.Delay` 0.5)
        (set `self.isAttacking` false)))
    (:`NewEnumerator3`
      (goto _label))))

(event `StopRunServer`
  ;[1 1 1] Run
  (`self.StopRunningMulticast`))

(event `RunServer`
  ;[1 1 1] Run
  (`self.RunMulticast`))

(event `RunMulticast`
  ;[1 1 1] Run
  (set `self.isRunning` true)
  (set `CharacterMovementComponent.MaxWalkSpeed` (`self.RunSpeed`) (`self.CharacterMovement`)))

(event `InputAction|Run`
  (params (Key :type "Key Structure"))
  ;[1 1 1] Run
  (:`Pressed`
    (`self.RunServer`))
  (:`Released`
    (`self.StopRunServer`)))

(event `StopRunningMulticast`
  ;[1 1 1] Run
  (set `self.isRunning` false)
  (set `CharacterMovementComponent.MaxWalkSpeed` (`self.WalkSpeed`) (`self.CharacterMovement`)))

(event `InputAxis|MoveRight`
  (params (AxisValue :type "Float (single-precision)"))
  (`self.AddMovementInput` (1.0 0.0 0.0) AxisValue))

(event `InputAxis|MoveUp`
  (params (AxisValue :type "Float (single-precision)"))
  (`self.AddMovementInput` (0.0 -1.0 0.0) AxisValue))

(event `self.ReceiveTick`
  (params (DeltaSeconds :type "Float (single-precision)"))
  (bind _returnvalue (`self.GetController`))
  (bind _returnvalue_2 (`self.GetController`))
  (`|ExecutionSequence`
    (:`then_0`
      (`parent.ReceiveTick` DeltaSeconds)
      (if (not (`self.IsMovementLocked`))
        (`/Engine/EditorBlueprintResources/StandardMacros.CompareFloat` (.x (`MovementComponent.Velocity` (`self.GetMovementComponent`)))
          (:`>`
            ;[0 0.4745 1] Look Right
            (`/Engine/EditorBlueprintResources/StandardMacros.IsValid` _returnvalue_2
              (:`Is Valid`
                (`Controller.SetControlRotation` _returnvalue_2 (`KismetMathLibrary.MakeRotator` 0.0)))))
          (:`<`
            ;[0 0.4745 1] Look Left
            (`/Engine/EditorBlueprintResources/StandardMacros.IsValid` _returnvalue
              (:`Is Valid`
                (`Controller.SetControlRotation` _returnvalue (`KismetMathLibrary.MakeRotator` 0.0 0.0 180.0))))))))))

(event `InputAction|Ability 1`
  (params (Key :type "Key Structure"))
  (bind _shoot (`self.Shoot`))
  (:`Pressed`
    (switch `/Game/Blueprints/ENUM_Clases` (`self.Class`)
      (:`NewEnumerator1`
        (`/Engine/EditorBlueprintResources/StandardMacros.IsValid` (`self.ActivatedGameplaAbility`)
          (:`Is Valid`
            (`/Game/Blueprints/Abilities/BP_GameplayAbility.DeactivateAbility` (`self.ActivatedGameplaAbility`))
            (set `self.isUsingAbility1` false)
            (`self.K2_DestroyActor` (`self.ActivatedGameplaAbility`)))
          (:`Is Not Valid`
            (set `self.isUsingAbility1` true)
            (bind _returnvalue (`|SpawnActorFromClass` "/Game/Blueprints/Abilities/GameplayAbility_Magician.GameplayAbility_Magician_C" (`self.GetTransform`) "Undefined" "OverrideRootScale" null "NewEnumerator0" 0.0 "NewEnumerator0" null))
            (bind _output_get (set `self.ActivatedGameplaAbility` _returnvalue))
            (`/Game/Blueprints/Abilities/BP_GameplayAbility.ActivateAbility` _output_get))))
      (:`NewEnumerator2`
        (if (!= (`self.isAttacking`) true)
          (set `self.isAttacking` true)
          (`KismetSystemLibrary.Delay` 0.5)
          (bind _returnvalue_2 (`|SpawnActorFromClass` "/Game/Blueprints/Actors/BP_Arrow.BP_Arrow_C" (`KismetMathLibrary.MakeTransform` (`SceneComponent.K2_GetComponentLocation` _shoot) (`SceneComponent.K2_GetComponentRotation` _shoot)) "Undefined" "OverrideRootScale" null null))
          (`SceneComponent.SetVisibility` (`/Game/Blueprints/Actors/BP_Arrow.PointLight` _returnvalue_2) true false)
          (`KismetSystemLibrary.Delay` 0.5)
          (set `self.isAttacking` false))))))

(event `self.ReceiveAnyDamage`
  (params (Damage :type "Float (single-precision)") (DamageType :type "DamageType Object Reference") (InstigatedBy :type "Controller Object Reference") (DamageCauser :type "Actor Object Reference"))
  (bind _output_get (set `self.Health` (- (`self.Health`) Damage)))
  (if (<= _output_get 0.0)
    (`KismetSystemLibrary.PrintString` "HAS MUERTO")))

(fn `OnRep_Class`
  (switch `/Game/Blueprints/ENUM_Clases` (`self.Class`)
    (:`NewEnumerator0`
      (`PaperZDAnimationComponent.SetAnimInstanceClass` (`self.AnimationComponent`) "/Game/Blueprints/Hero/ABP_Hero_Guardian.ABP_Hero_Guardian_C"))
    (:`NewEnumerator1`
      (`PaperZDAnimationComponent.SetAnimInstanceClass` (`self.AnimationComponent`) "/Game/Blueprints/Hero/ABP_HeroMagician.ABP_HeroMagician_C"))
    (:`NewEnumerator2`
      (`PaperZDAnimationComponent.SetAnimInstanceClass` (`self.AnimationComponent`) "/Game/Blueprints/Hero/ABP_Hero_Archer.ABP_Hero_Archer_C"))
    (:`NewEnumerator3`
      (`PaperZDAnimationComponent.SetAnimInstanceClass` (`self.AnimationComponent`) "/Game/Blueprints/Hero/ABP_Hero_Warrior.ABP_Hero_Warrior_C"))))

(fn `UserConstructionScript`)