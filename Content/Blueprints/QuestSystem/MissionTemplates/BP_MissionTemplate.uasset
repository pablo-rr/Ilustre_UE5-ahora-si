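; BP_MissionTemplate is a quest-system mission base actor that serves as a template for individual missions.
; On BeginPlay it binds MissionCompleted to its Completed event and prints a load message.
; On completion it prints a congratulation, tells the QuestManager to advance to the next objective and destroys itself.
; LoadDialogs is an empty event, apparently a hook for mission dialog loading.
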(event `self.ReceiveBeginPlay`
  (`|ExecutionSequence`
    (:`then_0`
      (add `self.Completed` (delegate `MissionCompleted`)))
    (:`then_2`
      (`KismetSystemLibrary.PrintText` (`|FormatText` "Loaded {load}" self)))))

(event `MissionCompleted`
  (`KismetSystemLibrary.PrintString` "Well done!")
  (`/Game/Blueprints/QuestSystem/BP_QuestManager.NextObjective` (`self.QuestManager`) null)
  (`self.K2_DestroyActor`))

(event `LoadDialogs`)

(fn `UserConstructionScript`)