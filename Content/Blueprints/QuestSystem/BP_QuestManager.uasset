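; Quest manager that starts a quest by ID and steps through its missions from DT_Quests, spawning each as an objective actor at the world origin.
; Each spawned objective receives a manager reference and the quest's starting dialog name.
; At the first objective and past the last, it loads the starting or ending dialog from DT_Dialogs into WG_Quest and calls DeleteCurrentObjective.
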(fn `LoadDialogs`
  (params (DialogName :type String) (Widget :type "UserWidget Object Reference"))
  (`KismetSystemLibrary.PrintString` DialogName)
  (bind _returnvalue (`|GetDataTableRow` "/Game/Blueprints/QuestSystem/DT_Dialogs.DT_Dialogs" (`KismetStringLibrary.Conv_StringToName` DialogName))
    (:`then`
      (bind _aswg_quest (cast `/Game/UI/WG_Quest` (`self.Widget`)))
      (set `/Game/UI/WG_Quest.DialogTable` _returnvalue _aswg_quest)
      (`/Game/UI/WG_Quest.HandleDialog` _aswg_quest))
    (:`RowNotFound`
      (`KismetSystemLibrary.PrintString` DialogName))))

(fn `LoadQuest`
  (params (Id :type Integer) (Widget :type "UserWidget Object Reference"))
  (set `self.Widget` Widget)
  (set `self.QuestId` Id)
  (set `self.ObjectiveIndex` -1)
  (`self.NextObjective` Widget)
  (bind _aswg_quest (cast `/Game/UI/WG_Quest` Widget))
  (set `/Game/UI/WG_Quest.QuestId` (`self.QuestId`) _aswg_quest))

(fn `NextObjective`
  (params (Widget :type "UserWidget Object Reference"))
  (set `self.ObjectiveIndex` (+ 1 (`self.ObjectiveIndex`)))
  (bind _returnvalue (`|GetDataTableRow` "/Game/Blueprints/QuestSystem/DT_Quests.DT_Quests" (`KismetStringLibrary.Conv_StringToName` (`KismetStringLibrary.Conv_IntToString` (`self.QuestId`))))
    (:`then`
      (bind (_id _name _missions _reward _startingdialogname _endingdialogname) (break `/Game/Blueprints/QuestSystem/S_Quest` _returnvalue))
      (bind _returnvalue_2 (`|SpawnActorFromClass` (`|GetArrayItem` _missions (`self.ObjectiveIndex`)) (`KismetMathLibrary.MakeTransform` (0.0 0.0 0.0)) "Undefined" "OverrideRootScale" null null))
      (`|ExecutionSequence`
        (:`then_0`
          (set `/Game/Blueprints/QuestSystem/MissionTemplates/BP_MissionTemplate.QuestManager` self _returnvalue_2))
        (:`then_1`
          (bind _output_get (set `/Game/Blueprints/QuestSystem/MissionTemplates/BP_MissionTemplate.DialogName` _startingdialogname _returnvalue_2)))
        (:`then_2`
          (if (<= (`self.ObjectiveIndex`) 0)
            (`self.LoadDialogs` _output_get Widget)
            (`self.DeleteCurrentObjective`)))
        (:`then_3`
          (if (>= (`self.ObjectiveIndex`) (`KismetArrayLibrary.Array_Length` _missions))
            (set `/Game/Blueprints/QuestSystem/MissionTemplates/BP_MissionTemplate.DialogName` _endingdialogname _returnvalue_2)
            (`self.LoadDialogs` _endingdialogname Widget)
            (`self.DeleteCurrentObjective`)))))))

(fn `UserConstructionScript`)