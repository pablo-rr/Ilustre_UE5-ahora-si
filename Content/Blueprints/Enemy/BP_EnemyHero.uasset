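; AI-controlled enemy hero character that runs the BT_Enemy behavior tree when possessed.
; Run and attack events follow a Server-to-Multicast pattern, switching walk speed or enabling the attack collision for a timed window.
; Unless movement is locked, Tick snaps controller yaw left or right from the sign of X and Y velocity.
; Player-style input, UI, cosmetic and wizard ability logic remains only as unconnected nodes.
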(event `self.ReceiveBeginPlay`
  (`|ExecutionSequence`
    (:`then_1`
      (set `self.RunSpeed` (* (`self.WalkSpeed`) 1.5)))
    (:`then_2`
      (`PrimitiveComponent.SetCollisionEnabled` (`self.AttackColision`) "NoCollision"))))

(event `self.ReceivePossessed`
  (params (NewController :type "Controller Object Reference"))
  (bind _asaicontroller (cast `AIController` NewController))
  (`AIController.RunBehaviorTree` _asaicontroller "/Game/AI/BT_Enemy.BT_Enemy"))

(event `StopRunServer`
  ;[1 1 1] Run
  (`self.StopRunningMulticast`))

(event `RunServer`
  ;[1 1 1] Run
  (`self.RunMulticast`))

(event `RunMulticast`
  ;[1 1 1] Run
  (set `self.isRunning` true)
  (set `CharacterMovementComponent.MaxWalkSpeed` (`self.RunSpeed`) (`self.CharacterMovement`)))

(event `InputAction|Run`
  (params (Key :type "Key Structure"))
  ;[1 1 1] Run
)

(event `StopRunningMulticast`
  ;[1 1 1] Run
  (set `self.isRunning` false)
  (set `CharacterMovementComponent.MaxWalkSpeed` (`self.WalkSpeed`) (`self.CharacterMovement`)))

(event `InputAxis|MoveRight`
  (params (AxisValue :type "Float (single-precision)")))

(event `InputAxis|MoveUp`
  (params (AxisValue :type "Float (single-precision)")))

(event `InputAction|Attack`
  (params (Key :type "Key Structure"))
  ;[1 1 1] Ataque Básico
)

(event `AttackServer`
  ;[1 1 1] Ataque Básico
  (`self.AttackMulticast`))

(event `AttackMulticast`
  (bind _attackcolision (`self.AttackColision`))
  ;[1 1 1] Ataque Básico
  (if (!= (`self.isAttacking`) true)
    (set `self.isAttacking` true)
    (`PrimitiveComponent.SetCollisionEnabled` _attackcolision "QueryAndPhysics")
    (`KismetSystemLibrary.Delay` (`self.delayAttack`))
    (set `self.isAttacking` false)
    (`PrimitiveComponent.SetCollisionEnabled` _attackcolision "NoCollision")))

(event `self.ReceiveTick`
  (params (DeltaSeconds :type "Float (single-precision)"))
  (bind _returnvalue (`self.GetController`))
  (bind _returnvalue_2 (`self.GetController`))
  (bind _returnvalue_3 (`self.GetController`))
  (bind _returnvalue_4 (`self.GetController`))
  (`parent.ReceiveTick` DeltaSeconds)
  (if (not (`self.IsMovementLocked`))
    (`|ExecutionSequence`
      (:`then_0`
        (`/Engine/EditorBlueprintResources/StandardMacros.CompareFloat` (.x (`MovementComponent.Velocity` (`self.GetMovementComponent`)))
          (:`>`
            ;[0 0.4745 1] Look Right
            (`/Engine/EditorBlueprintResources/StandardMacros.IsValid` _returnvalue
              (:`Is Valid`
                (`Controller.SetControlRotation` _returnvalue (`KismetMathLibrary.MakeRotator` 0.0)))))
          (:`<`
            ;[0 0.4745 1] Look Left
            (`/Engine/EditorBlueprintResources/StandardMacros.IsValid` _returnvalue_2
              (:`Is Valid`
                (`Controller.SetControlRotation` _returnvalue_2 (`KismetMathLibrary.MakeRotator` 0.0 0.0 180.0)))))))
      (:`then_1`
        (`/Engine/EditorBlueprintResources/StandardMacros.CompareFloat` (.y (`MovementComponent.Velocity` (`self.GetMovementComponent`)))
          (:`>`
            ;[0 0.4745 1] Look Right
            (`/Engine/EditorBlueprintResources/StandardMacros.IsValid` _returnvalue_4
              (:`Is Valid`
                (`Controller.SetControlRotation` _returnvalue_4 (`KismetMathLibrary.MakeRotator` 0.0)))))
          (:`<`
            ;[0 0.4745 1] Look Left
            (`/Engine/EditorBlueprintResources/StandardMacros.IsValid` _returnvalue_3
              (:`Is Valid`
                (`Controller.SetControlRotation` _returnvalue_3 (`KismetMathLibrary.MakeRotator` 0.0 0.0 180.0))))))))))

(event `InputAction|Ability 1`
  (params (Key :type "Key Structure")))

(fn `UserConstructionScript`)