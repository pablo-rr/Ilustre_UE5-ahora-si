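; BP_Enemy is a 2D enemy actor that flashes its Paper sprite red when another actor overlaps it.
; Overlap calls TakeDamageSV, which passes to TakeDamageMulticast for the flash, then calls OnDamage.
; The flash saves the current color, waits briefly, then resets to white rather than the saved color.
; No health is tracked, and the saved color's OnRep is empty.
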(event `self.ReceiveActorBeginOverlap`
  (params (OtherActor :type "Actor Object Reference"))
  (`self.TakeDamageSV`)
  (`self.OnDamage`))

(event `TakeDamageMulticast`
  (bind _papersprite (`self.PaperSprite`))
  (set `self.spriteColorPrevious` (`PaperSpriteComponent.SpriteColor` _papersprite))
  (`PaperSpriteComponent.SetSpriteColor` _papersprite (struct :`R` 1.0 :`A` 1.0))
  (`KismetSystemLibrary.Delay` 0.2)
  (`PaperSpriteComponent.SetSpriteColor` (`self.PaperSprite`) (struct :`R` 1.0 :`G` 1.0 :`B` 1.0 :`A` 1.0)))

(event `TakeDamageSV`
  (`self.TakeDamageMulticast`))

(fn `OnRep_spriteColorPrevious`)

(fn `UserConstructionScript`)