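; Actor component that tracks an actor's Health, starting at MaxHealth, and signals when it is healed, damaged, fully healed or fatally damaged.
; Heal and Damage adjust Health, fire their notifications, then clamp at the limit they approach.
; FullyHeal and FatallyDamage reuse them with MaxHealth as the amount.
; SetHealth assigns before computing the difference, so its notification and clamp branches never run.
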(event `self.ReceiveBeginPlay`
  (set `self.Health` (`self.MaxHealth`)))

(event `Heal`
  (params (Ammount :type Integer))
  ;[1 1 1] Increase the Health by the Ammount given, calls Healed and/or FullyHealed if health equals MaxHealth
  (set `self.Health` (+ Ammount (`self.Health`)))
  (`self.Healed` Ammount)
  (`self.CallFullyHealedIfNeeded`))

(event `Damage`
  (params (Ammount :type Integer))
  ;[1 1 1] Lower the Health by the Ammount given, calls Damaged and/or FatallyDamaged if health below 0
  (set `self.Health` (- (`self.Health`) Ammount))
  (`self.Damaged` Ammount)
  (`self.CallFatallyDamagedIfNeeded`))

(event `CallFullyHealedIfNeeded`
  ;[1 1 1] Will call FullyHealed if health above MaxHealth
  (if (>= (`self.Health`) (`self.MaxHealth`))
    (`|ExecutionSequence`
      (:`then_0`
        (set `self.Health` (`self.MaxHealth`)))
      (:`then_1`
        (`self.FullyHealed`)))))

(event `FullyHeal`
  ;[1 1 1] Set Health to MaxHealth, calls Healed and FullyHealed
  (`self.Heal` (`self.MaxHealth`)))

(event `CallFatallyDamagedIfNeeded`
  ;[1 1 1] Will call FatallyDamaged if health below 0
  (if (<= (`self.Health`) 0)
    (`|ExecutionSequence`
      (:`then_0`
        (set `self.Health` 0))
      (:`then_1`
        (`self.FatallyDamaged`)))))

(event `FatallyDamage`
  ;[1 1 1] Set health to 0, calls Damaged and FatallyDamaged
  (`self.Damage` (`self.MaxHealth`)))

(fn `SetHealth`
  (params (NewHealth :type Integer))
  (locals (HealthDifference :type Integer))
  ;[1 1 1] /* WARNING: Do not confuse with SetHealth for the Variable Health, this function MUST be used when if updating the Health to a set value */                                                                                                                                       Set Health to NewHealth and call Healed/Damaged and /or FullyHealed/FatallyDamaged if needed.
  (`|ExecutionSequence`
    (:`then_0`
      (set `self.Health` NewHealth))
    (:`then_1`
      (bind _output_get (set `local.HealthDifference` (- NewHealth (`self.Health`))))
      (`|ExecutionSequence`
        (:`then_0`
          (if (> _output_get 0)
            (`self.Healed` 0)
            (`self.CallFullyHealedIfNeeded`)))
        (:`then_1`
          (if (< _output_get 0)
            (`self.Damaged` 0)
            (`self.CallFatallyDamagedIfNeeded`)))))))