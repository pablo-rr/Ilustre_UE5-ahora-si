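; BP_TrampArrow is an arrow projectile actor built on a Paper2D sprite that damages whatever it overlaps.
; On BeginPlay it launches itself with a physics impulse along the sprite's forward vector and destroys itself after a short delay.
; An actor overlap applies damage to the other actor and destroys the arrow immediately.
; The hit event is empty, and its binding and an explosion emitter spawn are left unconnected.
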(event `self.ReceiveActorBeginOverlap`
  (params (OtherActor :type "Actor Object Reference"))
  (`GameplayStatics.ApplyDamage` OtherActor 10.0)
  (`self.K2_DestroyActor`))

(event `self.ReceiveBeginPlay`
  (bind _papersprite (`self.PaperSprite`))
  (`PrimitiveComponent.AddImpulse` _papersprite (* (`SceneComponent.GetForwardVector` _papersprite) 3000.0) "None" false)
  (`KismetSystemLibrary.Delay` 3.0)
  (`self.K2_DestroyActor`))

(event `OnActorHit_Event` :!signature `self.OnActorHit`
  (params (SelfActor :type "Actor Object Reference") (OtherActor :type "Actor Object Reference") (NormalImpulse :type "Vector Structure") (Hit :type "HitResult Structure (by ref)")))

(fn `UserConstructionScript`)