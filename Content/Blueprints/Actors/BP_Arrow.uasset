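; BP_Arrow is an arrow projectile actor that launches itself and spawns an explosion effect on overlap.
; BeginPlay applies a large forward impulse to its PaperSprite.
; On overlap, a visibility trace from the Cube places P_Explosion at the impact point; its end is the scaled forward vector, without the start location added.
; A second trace that sets the hit component's physics velocity never runs.
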(event `self.ReceiveBeginPlay`
  (bind _papersprite (`self.PaperSprite`))
  (`PrimitiveComponent.AddImpulse` _papersprite (* (`SceneComponent.GetForwardVector` _papersprite) 500000.0) "None" false))

(event `self.ReceiveActorBeginOverlap`
  (params (OtherActor :type "Actor Object Reference"))
  (bind _cube (`self.Cube`))
  (bind _outhit (`KismetSystemLibrary.LineTraceSingle` (`SceneComponent.K2_GetComponentLocation` _cube) (* (`SceneComponent.GetForwardVector` _cube) 200.0) "TraceTypeQuery1"))
  (`GameplayStatics.SpawnEmitterAtLocation` "/Game/Engine/StarterContent/Particles/P_Explosion.P_Explosion" (`.ImpactPoint` (`GameplayStatics.BreakHitResult` _outhit))))

(fn `UserConstructionScript`)