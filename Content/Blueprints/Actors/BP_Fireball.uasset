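; BP_Fireball is a projectile actor that damages enemy heroes on overlap.
; On BeginPlay it launches its PaperSprite forward with a physics impulse and destroys itself after a short delay.
; Overlapping a BP_EnemyHero of that exact class applies damage, spawns an explosion emitter at the enemy's capsule and destroys the fireball.
; The actor-hit handler is empty and its binding never runs.
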(event `self.ReceiveBeginPlay`
  (`PrimitiveComponent.AddImpulse` (`self.PaperSprite`) (* (`SceneComponent.GetForwardVector` (`self.PaperSprite`)) 2000.0) "None" false)
  (`KismetSystemLibrary.Delay` 3.0)
  (`self.K2_DestroyActor`))

(event `self.ReceiveActorBeginOverlap`
  (params (OtherActor :type "Actor Object Reference"))
  (bind _asbp_enemy_hero (cast `/Game/Blueprints/Enemy/BP_EnemyHero` OtherActor))
  (if (== (`GameplayStatics.GetObjectClass` OtherActor) "/Game/Blueprints/Enemy/BP_EnemyHero.BP_EnemyHero_C")
    (`GameplayStatics.ApplyDamage` OtherActor 60.0)
    (`/Engine/EditorBlueprintResources/StandardMacros.IsValid` OtherActor
      (:`Is Valid`
        (`GameplayStatics.SpawnEmitterAtLocation` "/Game/Engine/StarterContent/Particles/P_Explosion.P_Explosion" (`SceneComponent.K2_GetComponentLocation` (`Character.CapsuleComponent` _asbp_enemy_hero))))
      (:`Is Not Valid`
        _))
    (`self.K2_DestroyActor`)))

(event `OnActorHit_Event` :!signature `self.OnActorHit`
  (params (SelfActor :type "Actor Object Reference") (OtherActor :type "Actor Object Reference") (NormalImpulse :type "Vector Structure") (Hit :type "HitResult Structure (by ref)")))

(fn `UserConstructionScript`)