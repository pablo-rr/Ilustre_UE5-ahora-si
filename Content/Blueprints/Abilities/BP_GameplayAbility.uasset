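; BP_GameplayAbility is a base ability Blueprint that routes activation and deactivation by ability type.
; On BeginPlay it caches the player's BP_CustomHero and its ABP_Hero animation instance.
; ActivateAbility and DeactivateAbility switch on AbilityType and cast self to the matching child class, so the base knows its subclasses.
; Only the Magician case is wired, turning that child's light ability on and off.
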(event `self.ReceiveBeginPlay`
  (`self.CharacterRef`)
  (`self.ABPCharacterRef`))

(event `ActivateAbility`
  (switch `/Game/Blueprints/Abilities/GameplayAbilityType` (`self.AbilityType`)
    (:`NewEnumerator0`
      (bind _asgameplay_ability_magician (cast `/Game/Blueprints/Abilities/GameplayAbility_Magician` self))
      (`/Game/Blueprints/Abilities/GameplayAbility_Magician.ActivateLightAbility` _asgameplay_ability_magician))))

(event `DeactivateAbility`
  (switch `/Game/Blueprints/Abilities/GameplayAbilityType` (`self.AbilityType`)
    (:`NewEnumerator0`
      (bind _asgameplay_ability_magician (cast `/Game/Blueprints/Abilities/GameplayAbility_Magician` self))
      (`/Game/Blueprints/Abilities/GameplayAbility_Magician.DeactivateLightAbility` _asgameplay_ability_magician))))

(fn `ABPCharacterRef`
  (bind _asbp_custom_hero (cast `/Game/Blueprints/Hero/BP_CustomHero` (`GameplayStatics.GetPlayerCharacter` 0)))
  (bind _asabp_hero (cast `/Game/Blueprints/Hero/ABP_Hero` (`PaperZDAnimationComponent.AnimInstance` (`PaperZDCharacter.AnimationComponent` _asbp_custom_hero))))
  (set `self.ABP Hero Reference` _asabp_hero))

(fn `CharacterRef`
  (bind _asbp_custom_hero (cast `/Game/Blueprints/Hero/BP_CustomHero` (`GameplayStatics.GetPlayerCharacter` 0)))
  (set `self.CharRef` _asbp_custom_hero))

(fn `UserConstructionScript`)