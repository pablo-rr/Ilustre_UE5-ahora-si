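; GameplayAbility_Archer is an archer ability Blueprint that switches a light effect on the character on and off.
; On BeginPlay it calls functions to set up its character and animation Blueprint references.
; Activate and deactivate events switch on the archer ability type and, for Light Only, toggle the character's LightAbility component visibility with a debug print.
; An unconnected BP_Arrow spawn node never runs.
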(event `self.ReceiveBeginPlay`
  (`self.CharacterRef`)
  (`self.ABPCharacterRef`))

(event `ActivateLightAbility`
  (switch `/Game/Blueprints/Abilities/ArcherAbilityType` (`self.ArcherAbilityType`)
    (:`NewEnumerator0`
      (`KismetSystemLibrary.PrintString` "Flecha luz")
      (`SceneComponent.SetVisibility` (`/Game/Blueprints/Hero/BP_CustomHero.LightAbility` (`self.CharRef`)) true false))))

(event `DeactivateLightAbility`
  (switch `/Game/Blueprints/Abilities/ArcherAbilityType` (`self.ArcherAbilityType`)
    (:`NewEnumerator0`
      (`KismetSystemLibrary.PrintString` "Luz Apagada")
      (`SceneComponent.SetVisibility` (`/Game/Blueprints/Hero/BP_CustomHero.LightAbility` (`self.CharRef`)) false false))))

(fn `UserConstructionScript`
  (`parent.UserConstructionScript`))