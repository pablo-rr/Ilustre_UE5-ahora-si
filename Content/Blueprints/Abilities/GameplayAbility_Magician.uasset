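; Magician ability Blueprint that handles activation of a light ability on a Paper2D character.
; On BeginPlay it calls helpers for the character and ABP character references.
; When the ability type is Light Only, activation prints a debug message and sets the character sprite's flipbook to a sword attack animation.
; Deactivation is an empty stub, and the construction script only calls its parent.
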(event `self.ReceiveBeginPlay`
  (`self.CharacterRef`)
  (`self.ABPCharacterRef`))

(event `ActivateLightAbility`
  (switch `/Game/Blueprints/Abilities/MagicianAbilityType` (`self.MagicianAbilityType`)
    (:`NewEnumerator0`
      (`KismetSystemLibrary.PrintString` "Luz activada")
      (`PaperFlipbookComponent.SetFlipbook` (`PaperCharacter.Sprite` (`self.CharacterReference`)) "/Game/Sprites/CharacterTest/Attack/Sword/Anim_Atack_Sword1.Anim_Atack_Sword1"))))

(event `DeactivateLightAbility`)

(fn `UserConstructionScript`
  (`parent.UserConstructionScript`))