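; Guardian ability Blueprint that switches a light on the character on and off.
; On BeginPlay it runs the CharacterRef and ABPCharacterRef setup calls.
; Activate and deactivate events switch on GuardianAbilityType, with only the Light Only case implemented.
; That case toggles the visibility of the character's LightAbility component, tinting it cyan on activation.
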(event `self.ReceiveBeginPlay`
  (`self.CharacterRef`)
  (`self.ABPCharacterRef`))

(event `ActivateLightAbility`
  (bind _lightability (`/Game/Blueprints/Hero/BP_CustomHero.LightAbility` (`self.CharRef`)))
  (switch `/Game/Blueprints/Abilities/GuardianAbilityType` (`self.GuardianAbilityType`)
    (:`NewEnumerator0`
      (`SceneComponent.SetVisibility` _lightability true false)
      (`LightComponent.SetLightColor` _lightability (struct :`R` 0.196222 :`G` 0.683155 :`B` 0.734375 :`A` 1.0) true))))

(event `DeactivateLightAbility`
  (switch `/Game/Blueprints/Abilities/GuardianAbilityType` (`self.GuardianAbilityType`)
    (:`NewEnumerator0`
      (`SceneComponent.SetVisibility` (`/Game/Blueprints/Hero/BP_CustomHero.LightAbility` (`self.CharRef`)) false false))))

(fn `UserConstructionScript`
  (`parent.UserConstructionScript`))